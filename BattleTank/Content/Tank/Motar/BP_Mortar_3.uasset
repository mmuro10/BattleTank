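; BP_Mortar_3 is a mortar Blueprint in the Tank game, set up with an aimable barrel and turret and a health bar widget.
; On BeginPlay it passes its Barrel and Turret to the TankAiming component's Initialize.
; It then casts its widget component's user widget to WBP_HealthBar and sets itself as that bar's MyTank.
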(event `self.ReceiveBeginPlay`
  (`TankAimingComponent.Initialize` (`self.TankAiming`) (`self.Barrel`) (`self.Turret`))
  (`self.Initialize Health Bar`))

(fn `Initialize Health Bar`
  (bind _aswbp_health_bar (cast `/Game/UI/WBP_HealthBar` (`WidgetComponent.GetUserWidgetObject` (`self.Widget`))))
  (set `/Game/UI/WBP_HealthBar.MyTank` self _aswbp_health_bar)
  (return))

(fn `UserConstructionScript`)